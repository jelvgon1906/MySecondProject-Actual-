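; Player controller that moves its controlled pawn toward the mouse cursor while the ToogleInput action is held.
; Pressing and releasing the action toggles a HasClicked flag, which Tick reads to trace under the cursor on the Visibility channel and add movement input toward the hit location.
; BeginPlay also sets a Vida (health) value and prints it, with no further use in this graph.
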(event EventBeginPlay
  (bind _output_get (Variables|Default|SetVida 1e+02))
  (Development|PrintString (Utilities|String|ToString(Float) _output_get) true true "(R=1.000000,G=0.000000,B=0.819077,A=1.000000)"))

(event EventTick
  (params (DeltaSeconds :type Float%20%28single-precision%29))
  (bind _returnvalue (Pawn|GetControlledPawn))
  (if (Variables|Default|GethasClicked)
    (Pawn|Input|AddMovementInput _returnvalue (Math|Vector|GetUnitDirection(Vector) (Transformation|GetActorLocation _returnvalue) (.Location (Collision|BreakHitResult (.HitResult (Game|Player|GetHitResultUnderCursorbyChannel "TraceTypeQuery1" true))))) 1.0 false)))

(event Input|ActionEvents|InputActionToogleInput
  (params (Key :type Key%20Structure :default "None"))
  (:Pressed
    (Variables|Default|SethasClicked true))
  (:Released
    (Variables|Default|SethasClicked false)))

(fn ConstructionScript)